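; BP_AmbientLightTweaker is an actor that drives the light direction of an ambient gradient fresnel material setup.
; It writes LightDirection into the GradientFresnelParamCollection material parameter collection and aims an arrow component along it, on construction and every tick.
; When IsAnimating is set, tick also recomputes the direction by rolling a vertical vector over game time at RotationVelocity.
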(event EventTick
  (params (DeltaSeconds :type Float%20%28single-precision%29))
  (CallFunction|UpdateLightDirection)
  (if (Variables|LightDirection|GetIsAnimating)
    (Variables|LightDirection|SetLightDirection (Math|Vector|RotateVector "0, 0,100.000000" (Math|Rotator|MakeRotator (* (Utilities|Time|GetGameTimeinSeconds) (Variables|LightDirection|GetRotationVelocity)) 0.0 0.0)))))

(fn ConstructionScript
  (CallFunction|UpdateLightDirection))

(fn UpdateLightDirection
  (Rendering|Material|SetVectorParameterValue "/Game/BlockOut/Materials_Textures/AmbientFresnel/GradientFresnelParamCollection.GradientFresnelParamCollection" "LightDirection" (Math|Conversions|ToLinearColor(Vector) (Variables|LightDirection|GetLightDirection)) :!class /Script/Engine.KismetMaterialLibrary)
  (Transformation|SetRelativeRotation (Variables|Default|GetArrow1) (Math|Rotator|FindLookatRotation (Math|Vector|MakeVector 0.0 0.0 0.0) (Variables|LightDirection|GetLightDirection)) false false))