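; Demo actor that shows a skeletal mesh as an animated hologram, using a second depth-only mesh for depth culling.
; The construction script assigns the hologram and depth materials to the two skeletal meshes and toggles the depth mesh's visibility with DepthCullEnabled for demonstration.
; On BeginPlay both meshes start the same looping forward run animation.
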(event EventBeginPlay
  (bind _runfwdanim (Variables|Default|GetRunFwdAnim))
  (Components|Animation|PlayAnimation (Variables|BP_SK_Hologram|GetOpaqueSK) _runfwdanim true)
  (Components|Animation|PlayAnimation (Variables|BP_SK_Hologram|GetDepthOnlySK) _runfwdanim true))

(fn ConstructionScript
  ;[1 1 1] Set Depth-only Material
  (Rendering|Material|SetMaterial (Variables|BP_SK_Hologram|GetDepthOnlySK) 0 (Variables|Default|GetDepthMaterial))
  ;[1 1 1] Set Hologram Material
  (Rendering|Material|SetMaterial (Variables|BP_SK_Hologram|GetOpaqueSK) 0 (Variables|Default|GetHologramMaterial))
  ;[1 1 1] For Demoing purposes we can toggle depth culling
  (Rendering|SetVisibility (Variables|BP_SK_Hologram|GetDepthOnlySK) (Variables|Default|GetDepthCullEnabled) false))